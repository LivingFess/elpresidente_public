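; HUD class for a swipe-style card game that selects cards, applies the chosen side's effects to four faction stats (Industry, Army, Church, Eco) and counts score.
; When a card is removed, it draws a random regular card or, on game over, a DataTable card matching the failed faction and border, then advances the pawn.
; Aftermath applies stat changes with debug printing, or resets stats and score after game over.
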(event Custom|Get%20Regular%20Card
  ;[1 1 1] Получение обычной карты
  (CallFunction|FindRegularCard))

(event Custom|Game%20Over%20Event
  ;[1 1 1] Отладочное сообщение конца игры
  (Development|PrintString "1000-7"))

(event Custom|Aftermath
  (bind _aspawn_main (Utilities|GetPAWN))
  (bind _card_data (Variables|Default|GetCard%20Data))
  (bind _chosen_card_side (Variables|/Game/Blueprints/PAWN_Main.PAWN_Main_C|GetChosen%20Card%20Side _aspawn_main))
  (bind _returnvalue (Utilities|Select :Index _chosen_card_side :NewEnumerator0 (.ltpoints _card_data) :NewEnumerator1 (.rtpoints _card_data)))
  ;[1 1 1] Расчёт после уборки карты
  (if (Variables|Default|GetGame%20Over)
    (Utilities|ResetStats)
    (Variables|Default|SetGame%20Over false)
    (Variables|Default|SetCurrect%20Score 0)
    (else
      (Development|PrintString (Utilities|String|ToString(Text) (Utilities|Text|FormatText "Change : {1} ; {2}; {3}; {4};" (.1industry _returnvalue) (.2army _returnvalue) (.3church _returnvalue) (.4eco _returnvalue))) true true "(R=0.000000,G=1.000000,B=0.505014,A=1.000000)" 1e+01)
      (Utilities|UpdateStats (.1industry _returnvalue) (.2army _returnvalue) (.3church _returnvalue) (.4eco _returnvalue)))))

(event Custom|Card%20is%20Removed
  (if (Variables|Default|GetGame%20Over)
    (CallFunction|FindGameOverCard)
    (Default|NextCard (Utilities|GetPAWN))
    (else
      (CallFunction|FindRegularCard)
      (Math|Integer|IncrementInt (Variables|Default|GetCurrect%20Score)
        (:%20%20
          (Default|NextCard (Utilities|GetPAWN)))))))

(fn ConstructionScript)

(fn FindRegularCard
  (bind _outrownames (DataTable|GetDataTableRowNames "/Game/Data_Tables/Cards_Regular.Cards_Regular"))
  (bind _returnvalue (Utilities|GetDataTableRow "/Game/Data_Tables/Cards_Regular.Cards_Regular" (Utilities|Array|Get(acopy) _outrownames (Math|Random|RandomInteger (Utilities|Array|Length _outrownames))))
    (:then
      (Variables|Default|SetCard%20Data _returnvalue))
    (:RowNotFound
      (Development|PrintString "ОШИБКА. ОБЫЧНАЯ КАРТА НЕ НАЙДЕНА. (HUD_MAIN/Func:Find Regular Card)" true true "(R=1.000000,G=0.000000,B=0.013170,A=1.000000)" 1e+01)))
  (Default|SetupCardData (Variables|/Game/Blueprints/PAWN_Main.PAWN_Main_C|GetMainHUD (Utilities|GetPAWN)))
  (return))

(fn FindGameOverCard
  (bind _gameoverreason (Variables|Default|GetGameOverReason))
  (switch Utilities|FlowControl|Switch|SwitchonENUM_FactionID (.faction _gameoverreason)
    (:NewEnumerator0
      (if (.minborder? _gameoverreason)
        (Utilities|GetGameOverCardbyReason 1 2)
        (else
          (Utilities|GetGameOverCardbyReason 3 4))))
    (:NewEnumerator1
      (if (.minborder? _gameoverreason)
        (Utilities|GetGameOverCardbyReason 5 6)
        (else
          (Utilities|GetGameOverCardbyReason 7 8))))
    (:NewEnumerator2
      (if (.minborder? _gameoverreason)
        (Utilities|GetGameOverCardbyReason 9 10)
        (else
          (Utilities|GetGameOverCardbyReason 11 12))))
    (:NewEnumerator3
      (if (.minborder? _gameoverreason)
        (Utilities|GetGameOverCardbyReason 13 14)
        (else
          (Utilities|GetGameOverCardbyReason 15 16)))))
  (return))