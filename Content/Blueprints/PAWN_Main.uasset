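; Main pawn for a swipe-left-or-right card game, handling touch input, card animation and the main HUD widget.
; Dragging moves the card horizontally against a swipe threshold scaled to viewport width, with the start point trailing the finger beyond it.
; A qualifying release picks the side, notifies the HUD and animates the card away.
; Timelines drive card flips and text fades, with CardState gating input until the next card is ready.
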(event Custom|Show%20Card%20HUD
  (Default|GetRegularCard (Utilities|GetHUD))
  (Utilities|FlowControl|Delay 1.0)
  (bind _alpha (Timeline|HUD%20Show Play)
    (:Update
      (Default|UpdateCardHUDOpacity (Variables|Default|GetMainHUD) _alpha)
      (Components|Timeline|SetPlayRate (Variables|Default|GetTimeline_0) 2.4)
      (bind (_direction _card_x_scale _br _card_y_scale _shadow_opacity) (Timeline|Timeline_0 PlayFromStart)
        (:Update
          (Default|FlipCard (Variables|/Game/Widgets/W_MainHUD.W_MainHUD_C|GetW_Card (Variables|Default|GetMainHUD)) (Math|Float|Lerp 1.0 0.0 _br) (Math|Float|Lerp 0.0 1.0 _br) _card_x_scale _card_y_scale _shadow_opacity)
          (Variables|Default|SetCard%20State "NewEnumerator0")
          (Variables|Default|SetStart ""))))))

(event Custom|Start%20Card%20Move
  (bind _mainhud (Variables|Default|GetMainHUD))
  (bind _mainhud_2 (Variables|Default|GetMainHUD))
  (Components|Timeline|SetPlayRate (Variables|Default|GetCard%20Move%20Timeline) 3.0)
  (Default|Aftermath (Utilities|GetHUD))
  (bind (_direction _alpha_1 _alpha_2) (Timeline|Card%20Move%20Timeline PlayFromStart)
    (:Update
      (Default|MoveCard (Variables|/Game/Widgets/W_MainHUD.W_MainHUD_C|GetW_Card _mainhud) (Math|Float|Lerp 0.0 (Utilities|Select :Index (Variables|Default|GetChosen%20Card%20Side) :NewEnumerator0 -8e+02 :NewEnumerator1 8e+02) _alpha_1) 0.0 1.0 0.0)
      (Default|UpdateTextOpacity _mainhud (Math|Float|Lerp 1.0 0.0 _alpha_2) -315.0 0.0))
    (:Finished
      (Default|MoveCard (Variables|/Game/Widgets/W_MainHUD.W_MainHUD_C|GetW_Card _mainhud_2) 0.0 0.0 0.0 0.0)
      (Default|RestoreCardTransform _mainhud_2)
      (Utilities|FlowControl|Delay 1.0)
      (Default|CardIsRemoved (Utilities|GetHUD)))))

(event Custom|Next%20Card
  (bind _mainhud (Variables|Default|GetMainHUD))
  (Default|MoveCard (Variables|/Game/Widgets/W_MainHUD.W_MainHUD_C|GetW_Card (Variables|Default|GetMainHUD)) 0.0 0.0 1.0 0.0)
  (Components|Timeline|SetPlayRate (Variables|Default|GetCard%20Flip) 2.4)
  (bind (_direction _card_x_scale _br _card_y_scale _shadow_opacity _name_and_text_opacity) (Timeline|Card%20Flip PlayFromStart)
    (:Update
      (Default|FlipCard (Variables|/Game/Widgets/W_MainHUD.W_MainHUD_C|GetW_Card _mainhud) (Math|Float|Lerp 1.0 0.0 _br) (Math|Float|Lerp 0.0 1.0 _br) _card_x_scale _card_y_scale _shadow_opacity)
      (Default|UpdateTextOpacity _mainhud _name_and_text_opacity -315.0 0.0))
    (:Finished
      (Variables|Default|SetCard%20State "NewEnumerator0")
      (Variables|Default|SetStart ""))))

(event Custom|Update%20Location
  (bind _touch_vector (CallFunction|GetInputVector))
  (bind _swipe_lenght (Variables|Default|GetSwipe%20Lenght))
  (bind _swipe_lenght_2 (Variables|Default|GetSwipe%20Lenght))
  (bind _x (Math|Vector2D|BreakVector2D _touch_vector))
  (Default|UpdateTranslation (Variables|Default|GetMainHUD) (* (- (.x (Variables|Default|GetStart)) _x) -1.0))
  (if (> (* (- (.x (Variables|Default|GetStart)) _x) -1.0) _swipe_lenght_2)
    (Variables|Default|SetStart (Math|Vector2D|MakeVector2D (- _x _swipe_lenght) 0.0))
    (elif (< (* (- (.x (Variables|Default|GetStart)) _x) -1.0) (* _swipe_lenght_2 -1.0))
      (Variables|Default|SetStart (Math|Vector2D|MakeVector2D (+ _x _swipe_lenght) 0.0))
      (elif (< (Math|Float|Absolute(Float) (- (.x (Variables|Default|GetStart)) _x)) (- (Variables|Default|GetSwipe%20Lenght) (Variables|Default|GetAccept%20Distance)))
        (Variables|Default|SetLaunch%20Card false)))))

(event EventBeginPlay
  (bind _returnvalue (Viewport|GetViewportSize))
  (bind _returnvalue_2 (/ (.x _returnvalue) 1e+02))
  (bind _returnvalue_3 (* _returnvalue_2 2e+01))
  (Variables|/Script/Engine.PlayerController|SetbShowMouseCursor (Game|GetPlayerController 0) true)
  (Utilities|FlowControl|Delay 0.3)
  (bind _output_get (Variables|Default|SetSwipe%20Lenght _returnvalue_3))
  (if (== _returnvalue_3 0.0)
    (Variables|Default|SetSwipe%20Lenght 1.2e+02))
  (bind _returnvalue_4 (UserInterface|CreateWidget "/Game/Widgets/W_MainHUD.W_MainHUD_C" 0 _output_get))
  (bind _output_get_2 (Variables|Default|SetMainHUD _returnvalue_4))
  (UserInterface|Viewport|AddtoViewport _output_get_2 2))

(event Input|KeyboardEvents|Escape
  (params (Key :type Key%20Structure :default "None"))
  (:Pressed
    (Game|QuitGame 0 "Quit" false)))

(event Input|TouchEvents|InputTouch
  (params (Location :type Vector) (FingerIndex :type ETouchIndex%20Enum))
  (bind _touch_vector (CallFunction|GetInputVector))
  (:Pressed
    (switch Utilities|FlowControl|Switch|SwitchonENUM_CardState (Variables|Default|GetCard%20State)
      (:NewEnumerator0
        (switch Utilities|FlowControl|Switch|SwitchonETouchIndex FingerIndex
          (:Touch1
            (Variables|Default|SetPressed true)
            (Variables|Default|SetStart _touch_vector)
            (CallFunction|UpdateLocation :!label _label)
            (Timeline|Timeline_1 Stop
              (:Update
                (CallFunction|UpdateLocation))))))))
  (:Released
    (switch Utilities|FlowControl|Switch|SwitchonENUM_CardState (Variables|Default|GetCard%20State)
      (:NewEnumerator0
        (switch Utilities|FlowControl|Switch|SwitchonETouchIndex FingerIndex
          (:Touch1
            (if (Variables|Default|GetPressed)
              (Variables|Default|SetPressed false)
              (if (Variables|Default|GetLaunch%20Card)
                (Variables|Default|SetCard%20State "NewEnumerator1")
                (CallFunction|CheckSide)
                (CallFunction|StartCardMove)
                (Variables|Default|SetLaunch%20Card false)
                (else
                  (Timeline|Timeline_1 PlayFromStart)))))))))
  (:Moved
    (switch Utilities|FlowControl|Switch|SwitchonENUM_CardState (Variables|Default|GetCard%20State)
      (:NewEnumerator0
        (switch Utilities|FlowControl|Switch|SwitchonETouchIndex FingerIndex
          (:Touch1
            (if (Variables|Default|GetPressed)
              (if (> (Math|Vector2D|Vector2DLength (- (Variables|Default|GetStart) _touch_vector)) (Variables|Default|GetSwipe%20Lenght))
                (Variables|Default|SetLaunch%20Card true)
                (goto _label)
                (else
                  (Variables|Default|SetLaunch%20Card false)
                  (goto _label))))))))))

(fn ConstructionScript)

(fn GetInputVector
  (bind _returnvalue (Game|GetPlayerController 0))
  (bind (_locationx _locationy) (Class|PlayerController|GetInputTouchState _returnvalue "Touch1"))
  (return (Math|Vector2D|MakeVector2D _locationx _locationy)))

(fn CheckSide
  (if (< (* (- (.x (Variables|Default|GetStart)) (.X (Math|Vector2D|BreakVector2D (CallFunction|GetInputVector)))) -1.0) 0.0)
    (Variables|Default|SetChosen%20Card%20Side "NewEnumerator0")
    (return)
    (else
      (Variables|Default|SetChosen%20Card%20Side "NewEnumerator1")
      (return))))